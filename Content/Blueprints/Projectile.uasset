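; Physics-driven projectile actor that is launched by force and removes itself shortly after coming to rest.
; Shoot enables collision and physics simulation on the static mesh, then applies the given force to it.
; Tick watches the mesh velocity: any movement marks it airborne, and a later near-stop sets a short lifespan once, guarded by the Dying flag.
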(event `self.ReceiveBeginPlay`
  (set `self.Airborne` false)
  (set `self.Dying` false))

(event `self.ReceiveTick`
  (params (DeltaSeconds :type "Float (single-precision)"))
  (bind _returnvalue (`KismetMathLibrary.VSize` (`SceneComponent.GetComponentVelocity` (`self.StaticMesh`))))
  (if (`self.Airborne`)
    ;[1 1 1] Airborne
    (`/Engine/EditorBlueprintResources/StandardMacros.CompareFloat` _returnvalue 0.1
      (:`<`
        (if (not (`self.Dying`))
          (`self.SetLifeSpan` 1.0)
          (set `self.Dying` true))))
    (else
      (`/Engine/EditorBlueprintResources/StandardMacros.CompareFloat` _returnvalue
        (:`>`
          (set `self.Airborne` true))))))

(fn `Shoot`
  (params (Force :type "Vector Structure"))
  (bind _staticmesh (`self.StaticMesh`))
  (`PrimitiveComponent.SetCollisionEnabled` _staticmesh "QueryAndPhysics")
  (`PrimitiveComponent.SetSimulatePhysics` _staticmesh true)
  (`PrimitiveComponent.AddForce` _staticmesh Force "None" false))

(fn `UserConstructionScript`)