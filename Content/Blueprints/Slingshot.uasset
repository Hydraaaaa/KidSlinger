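; Player slingshot that fires projectiles from a queue, with axis-driven aim and hold-to-charge power.
; Holding Shoot builds power on Tick up to a maximum and stretches a power sprite; releasing launches the projectile along AimDirection.
; While projectiles remain, it spawns the next and points its spawned Camera at the shot; the next Shoot release returns the camera and re-arms.
; An aim-angle clamp exists but is unconnected.
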(event `self.ReceiveBeginPlay`
  ;[1 1 1] BeginPlay
  (bind _spawnedactor (`self.SpawnProjectile`))
  (set `self.CurrentProjectile` _spawnedactor)
  (bind _returnvalue (`|SpawnActorFromClass` "/Game/Blueprints/Camera.Camera_C" (`self.GetTransform`) "Undefined" "OverrideRootScale"))
  (`PlayerController.SetViewTargetWithBlend` (`GameplayStatics.GetPlayerController` 0) _returnvalue 0.0 "VTBlend_Linear" 0.0 false)
  (bind _output_get (set `self.Camera` _returnvalue))
  (set `/Game/Blueprints/Camera.FollowTarget` self _output_get)
  (set `/Game/Blueprints/Camera.Player` self _output_get)
  (set `self.Ready` true))

(event `InputAction|Shoot`
  (params (Key :type "Key Structure" :default "AnyKey"))
  (bind _ready (`self.Ready`))
  ;[1 1 1] Shoot
  (:`Pressed`
    (if _ready
      (set `self.ChargingUp` true)))
  (:`Released`
    (if _ready
      (set `self.ChargingUp` false)
      (bind _asprojectile (cast `/Game/Blueprints/Projectile` (`self.CurrentProjectile`)))
      (`/Game/Blueprints/Projectile.Shoot` _asprojectile (* (`SceneComponent.GetForwardVector` (`self.AimDirection`)) (`self.CurrentFirePower`)))
      (`/Engine/EditorBlueprintResources/StandardMacros.CompareInt` (`KismetArrayLibrary.Array_Length` (`self.Projectiles`))
        (:`>`
          (set `/Game/Blueprints/Camera.FollowTarget` (`self.CurrentProjectile`) (`self.Camera`))
          (bind _spawnedactor (`self.SpawnProjectile`))
          (set `self.CurrentProjectile` _spawnedactor)
          (set `self.CurrentFirePower` 0.0)
          (set `self.Ready` false)))
      (else
        (set `self.Ready` true)
        (set `/Game/Blueprints/Camera.FollowTarget` self (`self.Camera`))))))

(event `InputAxis|Turn`
  (params (AxisValue :type "Float (single-precision)"))
  ;[1 1 1] Turn
  (`SceneComponent.K2_AddWorldRotation` (`self.AimDirection`) (`KismetMathLibrary.MakeRotator` AxisValue) false false))

(event `self.ReceiveTick`
  (params (DeltaSeconds :type "Float (single-precision)"))
  (bind _maxfirepower (`self.MaxFirePower`))
  ;[1 1 1] Charge Up
  (if (`self.ChargingUp`)
    (bind _output_get (set `self.CurrentFirePower` (+ (* DeltaSeconds (/ (`self.MaxFirePower`) (`self.ChargeTime`))) (`self.CurrentFirePower`))))
    (`/Engine/EditorBlueprintResources/StandardMacros.CompareFloat` _output_get _maxfirepower
      (:`>`
        (set `self.CurrentFirePower` _maxfirepower))
      (:`==`
        _)
      (:`<`
        _))
    (`SceneComponent.SetWorldScale3D` (`self.Power Sprite`) (`KismetMathLibrary.MakeVector` 1.0 1.0 (`KismetMathLibrary.Lerp` 0.0 4.0 (/ (`self.CurrentFirePower`) (`self.MaxFirePower`)))))))

(fn `SpawnProjectile`
  (returns (SpawnedActor :type "/Game/Blueprints/Projectile Object Reference"))
  (bind _projectiles (`self.Projectiles`))
  (bind _returnvalue (`|SpawnActorFromClass` (`KismetArrayLibrary.Array_Get` _projectiles) (`SceneComponent.K2_GetComponentToWorld` (`self.AimDirection`)) "Undefined" "OverrideRootScale"))
  (`KismetArrayLibrary.Array_Remove` _projectiles)
  (`self.K2_AddActorWorldRotation` _returnvalue (struct :`Yaw` -90.0) false false)
  (bind _asprojectile (cast `/Game/Blueprints/Projectile` _returnvalue))
  (`PrimitiveComponent.SetCollisionEnabled` (`/Game/Blueprints/Projectile.StaticMesh` _asprojectile) "NoCollision")
  (return _asprojectile))

(fn `UserConstructionScript`)