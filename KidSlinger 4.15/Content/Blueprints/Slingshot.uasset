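; Player-controlled slingshot that launches projectiles from a queue of classes and spawns its own follow camera at BeginPlay.
; Turn input rotates AimDirection within a clamped roll, while holding Shoot builds fire power on Tick up to a maximum.
; Release fires the loaded projectile along the aim vector.
; If the queue still has entries, the camera then follows that shot, SpawnProjectile loads the next with collision disabled, and power resets.
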(event `self.ReceiveBeginPlay`
  ;[1 1 1] BeginPlay
  (bind _spawnedactor (`self.SpawnProjectile`))
  (set `self.CurrentProjectile` _spawnedactor)
  (bind _returnvalue (`|SpawnActorFromClass` "/Game/Blueprints/Camera.Camera_C" (`self.GetTransform`) "Undefined" "OverrideRootScale"))
  (`PlayerController.SetViewTargetWithBlend` (`GameplayStatics.GetPlayerController` 0) _returnvalue 0.0 "VTBlend_Linear" 0.0 false)
  (bind _output_get (set `self.Camera` _returnvalue))
  (set `/Game/Blueprints/Camera.FollowTarget` self _output_get)
  (set `/Game/Blueprints/Camera.Player` self _output_get))

(event `InputAction|Shoot`
  (params (Key :type "Key Structure" :default "AnyKey"))
  ;[1 1 1] Shoot
  (:`Pressed`
    (set `self.ChargingUp` true)
    (`KismetSystemLibrary.PrintString` "Charging" true true (struct :`A` 1.0) 5.0))
  (:`Released`
    (set `self.ChargingUp` false)
    (bind _asprojectile (cast `/Game/Blueprints/Projectile` (`self.CurrentProjectile`)))
    (`/Game/Blueprints/Projectile.Shoot` _asprojectile (* (`SceneComponent.GetForwardVector` (`self.AimDirection`)) (`self.CurrentFirePower`)))
    (`/Engine/EditorBlueprintResources/StandardMacros.CompareInt` (`KismetArrayLibrary.Array_Length` (`self.Projectiles`))
      (:`>`
        (set `/Game/Blueprints/Camera.FollowTarget` (`self.CurrentProjectile`) (`self.Camera`))
        (bind _spawnedactor (`self.SpawnProjectile`))
        (set `self.CurrentProjectile` _spawnedactor)
        (set `self.CurrentFirePower` 0.0)))))

(event `InputAxis|Turn`
  (params (AxisValue :type "Float (single-precision)"))
  (bind _aimdirection (`self.AimDirection`))
  ;[1 1 1] Turn
  (`SceneComponent.K2_AddWorldRotation` _aimdirection (`KismetMathLibrary.MakeRotator` AxisValue) false false)
  (`SceneComponent.K2_SetWorldRotation` _aimdirection (`KismetMathLibrary.MakeRotator` (`KismetMathLibrary.ClampAngle` (.roll (`SceneComponent.K2_GetComponentRotation` _aimdirection)) -45.0 85.0) (.pitch (`SceneComponent.K2_GetComponentRotation` _aimdirection)) (.yaw (`SceneComponent.K2_GetComponentRotation` _aimdirection))) false false))

(event `self.ReceiveTick`
  (params (DeltaSeconds :type "Float (single-precision)"))
  (bind _maxfirepower (`self.MaxFirePower`))
  ;[1 1 1] Charge Up
  (if (`self.ChargingUp`)
    (bind _output_get (set `self.CurrentFirePower` (+ (* DeltaSeconds (/ (`self.MaxFirePower`) (`self.ChargeTime`))) (`self.CurrentFirePower`))))
    (`/Engine/EditorBlueprintResources/StandardMacros.CompareFloat` _output_get _maxfirepower
      (:`>`
        (set `self.CurrentFirePower` _maxfirepower)))))

(fn `SpawnProjectile`
  (returns (SpawnedActor :type "/Game/Blueprints/Projectile Object Reference"))
  (bind _projectiles (`self.Projectiles`))
  (bind _returnvalue (`|SpawnActorFromClass` (`KismetArrayLibrary.Array_Get` _projectiles) (`KismetMathLibrary.MakeTransform` (.location (`SceneComponent.K2_GetComponentToWorld` (`self.AimDirection`))) (.rotation (`SceneComponent.K2_GetComponentToWorld` (`self.AimDirection`))) (0.5 0.5 0.5)) "Undefined" "OverrideRootScale"))
  (`KismetArrayLibrary.Array_Remove` _projectiles)
  (`self.K2_AddActorWorldRotation` _returnvalue (struct :`Yaw` -90.0) false false)
  (bind _asprojectile (cast `/Game/Blueprints/Projectile` _returnvalue))
  (`PrimitiveComponent.SetCollisionEnabled` (`/Game/Blueprints/Projectile.StaticMesh` _asprojectile) "NoCollision")
  (return _asprojectile))

(fn `UserConstructionScript`)